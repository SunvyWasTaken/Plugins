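; Game instance that manages the game's save slots through a master index save (SG_Main).
; On Init it loads or creates that master save, then caches its save list and current game name.
; Functions create SG_Game slots, delete them or set the current game, writing each change back to the master save.
; Creating a name that already exists quits the game, and deleting the current game clears that selection.
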(event `self.ReceiveInit`
  (`self.F_GetMainSave`)
  (`self.F_LoadData`))

(fn `F_CreatSaveGame`
  (params (SaveName :type String))
  (bind _returnvalue (`GameplayStatics.DoesSaveGameExist` SaveName))
  (if _returnvalue
    (`KismetSystemLibrary.QuitGame` null "Quit" true)
    (return)
    (else
      (bind _returnvalue_2 (`GameplayStatics.CreateSaveGameObject` "/Game/SaveGame/Blueprint/SG_Game.SG_Game_C"))
      (`GameplayStatics.SaveGameToSlot` _returnvalue_2 (`local.SaveName`))
      (`KismetArrayLibrary.Array_AddUnique` (`self.ListeSaveGame`) (`local.SaveName`))
      (set `/Game/MainSave/Blueprint/SG_Main.SaveList` (`self.ListeSaveGame`) (`self.SaveGameMainRef`))
      (`GameplayStatics.SaveGameToSlot` (`self.SaveGameMainRef`) (`self.SaveNameMain`))
      (return))))

(fn `F_GetMainSave`
  (bind _returnvalue (`GameplayStatics.DoesSaveGameExist` (`self.SaveNameMain`)))
  (if _returnvalue
    (bind _returnvalue_2 (`GameplayStatics.LoadGameFromSlot` (`self.SaveNameMain`)))
    (bind _assg_main (cast `/Game/MainSave/Blueprint/SG_Main` _returnvalue_2))
    (set `self.SaveGameMainRef` _assg_main)
    (return)
    (else
      (bind _returnvalue_3 (`GameplayStatics.CreateSaveGameObject` "/Game/MainSave/Blueprint/SG_Main.SG_Main_C"))
      (bind _output_get (set `self.SaveGameMainRef` _returnvalue_3))
      (`GameplayStatics.SaveGameToSlot` _output_get (`self.SaveNameMain`))
      (return))))

(fn `F_LoadData`
  (bind _savegamemainref (`self.SaveGameMainRef`))
  (set `self.ListeSaveGame` (`/Game/MainSave/Blueprint/SG_Main.SaveList` _savegamemainref))
  (set `self.CurrentGame` (`/Game/MainSave/Blueprint/SG_Main.CurrentGame` _savegamemainref))
  (return))

(fn `F_RemoveSave`
  (params (Item :type "String (by ref)"))
  (bind _savegamemainref (`self.SaveGameMainRef`))
  (`KismetArrayLibrary.Array_RemoveItem` (`self.ListeSaveGame`) Item) ; Remove de la liste dans\nle Game instance
  (`GameplayStatics.DeleteGameInSlot` Item)
  (set `/Game/MainSave/Blueprint/SG_Main.SaveList` (`self.ListeSaveGame`) _savegamemainref)
  (`GameplayStatics.SaveGameToSlot` _savegamemainref (`self.SaveNameMain`))
  (if (`KismetStringLibrary.EqualEqual_StrStr` (`local.Item`) (`self.CurrentGame`))
    (`self.F_SetCurrentGame` "")
    (return)
    (else
      (return))))

(fn `F_SetCurrentGame`
  (params (CurrentGame :type String))
  (bind _output_get (set `self.CurrentGame` CurrentGame))
  (set `/Game/MainSave/Blueprint/SG_Main.CurrentGame` _output_get (`self.SaveGameMainRef`))
  (`GameplayStatics.SaveGameToSlot` (`self.SaveGameMainRef`) (`self.SaveNameMain`))
  (return))