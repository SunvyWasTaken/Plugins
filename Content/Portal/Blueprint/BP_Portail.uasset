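; Portal actor whose plane displays the cube capture of another actor, referenced by TextureRenderTarget.
; On BeginPlay or GetMat it creates a runtime cube render target for its own scene capture, then feeds the referenced actor's cube texture into a dynamic CRT camera material on the plane.
; ToggleCamera flips between the CRT camera and cube materials, reapplying that texture each time.
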(event `GetMat`
  (bind _returnvalue (`|GenericCreateObject` "/Script/Engine.TextureRenderTargetCube" (`self.SceneCaptureComponentCube`) :!label _label))
  (bind _output_get (set `self.TextureRenderCube` _returnvalue))
  (set `SceneCaptureComponentCube.TextureTarget` _output_get (`self.SceneCaptureComponentCube`))
  (bind _texturerendertarget (`self.TextureRenderTarget`)
    (:`then`
      (bind _returnvalue_2 (`PrimitiveComponent.CreateDynamicMaterialInstance` (`self.Plane`) 0 "/Game/Portal/Material/CRT_Camera_Mat.CRT_Camera_Mat" "None"))
      (`MaterialInstanceDynamic.SetTextureParameterValue` _returnvalue_2 "Param" (`/Game/Portal/Blueprint/BP_Portail.TextureRenderCube` _texturerendertarget)))
    (:`else`)))

(event `self.ReceiveBeginPlay`
  (goto _label))

(event `ToggleCamera`
  (set `self.Camera` (not (`self.Camera`)))
  (bind _texturerendertarget (`self.TextureRenderTarget`)
    (:`then`
      (bind _returnvalue (`PrimitiveComponent.CreateDynamicMaterialInstance` (`self.Plane`) 0 (select `bool` (`self.Camera`) :`false` "/Game/Geometry/Meshes/CubeMaterial.CubeMaterial" :`true` "/Game/Portal/Material/CRT_Camera_Mat.CRT_Camera_Mat" :!type "MaterialInterface Object Reference") "None"))
      (`MaterialInstanceDynamic.SetTextureParameterValue` _returnvalue "Param" (`/Game/Portal/Blueprint/BP_Portail.TextureRenderCube` _texturerendertarget)))
    (:`else`)))

(fn `UserConstructionScript`)