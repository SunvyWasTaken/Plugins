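; GM_Game is the game mode that loads and saves the active save slot and adds the WBP_Interface widget at start.
; On BeginPlay it reads the slot name from GI_GameInstance and loads its SG_Game, quitting the game if none exists.
; A load step copies saved values unless the save is flagged empty.
; Functions adjust the example counter NbrEssais, and FSave writes it back to the slot, clearing the empty flag.
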(event `self.ReceiveBeginPlay`
  (`self.F_PreLoad`)
  (`self.F_Load`)
  (bind _returnvalue (`|CreateWidget` "/Game/SaveGame/Widget/WBP_Interface.WBP_Interface_C"))
  (`UserWidget.AddToViewport` _returnvalue 0))

(fn `F_AddNbr`
  (`/Engine/EditorBlueprintResources/StandardMacros.IncrementInt` (`self.NbrEssais`)
    (:`  `
      (return))))

(fn `F_Load`
  (if (not (`/Game/SaveGame/Blueprint/SG_Game.bIsEmptySave` (`self.SaveGameRef`)))
    ;[1 1 1] Get all the variable from the save game here
    (set `self.NbrEssais` (`/Game/SaveGame/Blueprint/SG_Game.Nbr` (`self.SaveGameRef`)))
    (return)
    (else
      (return) ; If it's Empty/NewSave Game Run with default Value
    )))

(fn `F_NegateNbr`
  (`/Engine/EditorBlueprintResources/StandardMacros.DecrementInt` (`self.NbrEssais`)
    (:`  `
      (return))))

(fn `F_PreLoad`
  ;[1 1 1] Normaly you don't need to thouch this function. U are supposed to load your varible on the function F_Load
  (bind _asgi_game_instance (cast `/Game/MainSave/Blueprint/GI_GameInstance` (`GameplayStatics.GetGameInstance`)))
  (bind _currentgame (`/Game/MainSave/Blueprint/GI_GameInstance.CurrentGame` _asgi_game_instance))
  (set `self.CurrentSave` _currentgame)
  (bind _returnvalue (`GameplayStatics.DoesSaveGameExist` _currentgame))
  (if _returnvalue
    (bind _returnvalue_2 (`GameplayStatics.LoadGameFromSlot` _currentgame))
    (bind _assg_game (cast `/Game/SaveGame/Blueprint/SG_Game` _returnvalue_2))
    (set `self.SaveGameRef` _assg_game)
    (return)
    (else
      (`KismetSystemLibrary.QuitGame` null "Quit") ; Close the game if there a error on the save
      (return))))

(fn `F_Save`
  (bind _savegameref (`self.SaveGameRef`))
  (set `/Game/SaveGame/Blueprint/SG_Game.bIsEmptySave` false _savegameref)
  (set `/Game/SaveGame/Blueprint/SG_Game.Nbr` (`self.NbrEssais`) _savegameref) ; Use for the Overview u can delete than
  ;[1 1 1] This node need to be the last when u save ur game
  (`GameplayStatics.SaveGameToSlot` (`self.SaveGameRef`) (`self.CurrentSave`))
  (return))

(fn `UserConstructionScript`)